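; BP_MyGameManager is an actor that tracks the game state (Running, Win, Lose or Abandon) and switches the matching UI.
; Init has BP_MyGameMode create the UI, then sets the state to Running.
; On a state change, SetState hides the UI, then either hides the mouse for Running or shows the end widget and mouse.
; ResetGame restarts by reopening the current level by name.
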(event EventBeginPlay)

(event Collision|EventActorBeginOverlap
  (params (OtherActor :type Actor%20Object%20Reference)))

(event EventTick
  (params (DeltaSeconds :type Float%20%28single-precision%29)))

(fn ConstructionScript)

(fn Init
  (bind _asbp_my_game_mode (Utilities|Casting|CastToBP_MyGameMode (Game|GetGameMode)))
  (Default|CreateUI _asbp_my_game_mode)
  (CallFunction|SetState "NewEnumerator0"))

(fn SetState
  (params (New%20State :type E_MyGameStates%20Enum :default "NewEnumerator0"))
  (if (Utilities|Enum|NotEqual(Enum) New%20State (Variables|Default|GetCurrent%20Game%20State))
    (CallFunction|HideUI)
    (bind _output_get (Variables|Default|SetCurrent%20Game%20State New%20State))
    (switch Utilities|FlowControl|Switch|SwitchonE_MyGameStates _output_get
      (:NewEnumerator0
        (CallFunction|ShowMouse false))
      (:NewEnumerator1
        (Widget|SetVisibility (Variables|Default|GetWidget_Win) "Visible")
        (CallFunction|ShowMouse true :!label _label))
      (:NewEnumerator2
        (Widget|SetVisibility (Variables|Default|GetWidget_Lose) "Visible")
        (goto _label))
      (:NewEnumerator3
        (Widget|SetVisibility (Variables|Default|GetWidget_Abandon) "Visible")
        (goto _label)))))

(fn GetState
  (return (Variables|Default|GetCurrent%20Game%20State)))

(fn ResetGame
  (bind _returnvalue (Game|GetCurrentLevelName true))
  (Game|OpenLevel(byName) (Utilities|String|StringToName _returnvalue)))